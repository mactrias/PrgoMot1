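; Fire trap that ignites and repeatedly damages the third-person character while it stands inside the collider.
; Overlap activates the fire effect and starts a looping timer that applies damage through the character's BPCLife component.
; A true damage result triggers death: input off, death montage, game-over widget and UI-only mouse control.
; Death or exit clears the timer by re-setting it to zero time; exit also extinguishes the fire after a delay.
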(event `self.Collider.OnComponentBeginOverlap`
  (params (OverlappedComponent :type "PrimitiveComponent Object Reference") (OtherActor :type "Actor Object Reference") (OtherComp :type "PrimitiveComponent Object Reference") (OtherBodyIndex :type Integer) (bFromSweep :type Boolean) (SweepResult :type "HitResult Structure (by ref)"))
  (bind _asbp_third_person_character (cast `/Game/ThirdPerson/Blueprints/BP_ThirdPersonCharacter` OtherActor))
  (`ActorComponent.Activate` (`self.NS_Fire`) false)
  (`KismetSystemLibrary.K2_SetTimerDelegate` (delegate `CustomEvent_0`) 0.5 true))

(event `CustomEvent_0`
  (bind _returnvalue (`GameplayStatics.GetPlayerController` 0))
  (bind _isdead (`/Game/ThirdPerson/Blueprints/BPC_life.RecibeDamage` (`/Game/ThirdPerson/Blueprints/BP_ThirdPersonCharacter.BPC_life` (stale `self.Collider.OnComponentBeginOverlap` _asbp_third_person_character)) 5.0))
  (if _isdead
    (`self.DisableInput` (stale `self.Collider.OnComponentBeginOverlap` _asbp_third_person_character) null)
    (`KismetSystemLibrary.K2_SetTimerDelegate` (delegate `CustomEvent_0`))
    (`Character.PlayAnimMontage` (stale `self.Collider.OnComponentBeginOverlap` _asbp_third_person_character) "/Game/Assets/character/Death_Montage.Death_Montage" 1.0 "None")
    (bind _returnvalue_2 (`|CreateWidget` "/Game/matlevel/GAmeOver/WGameOver.WGameOver_C"))
    (`UserWidget.AddToViewport` _returnvalue_2 0)
    (set `PlayerController.bShowMouseCursor` true _returnvalue)
    (`WidgetBlueprintLibrary.SetInputMode_UIOnlyEx` _returnvalue _returnvalue_2)))

(event `self.Collider.OnComponentEndOverlap`
  (params (OverlappedComponent :type "PrimitiveComponent Object Reference") (OtherActor :type "Actor Object Reference") (OtherComp :type "PrimitiveComponent Object Reference") (OtherBodyIndex :type Integer))
  (cast `/Game/ThirdPerson/Blueprints/BP_ThirdPersonCharacter` OtherActor)
  (`KismetSystemLibrary.K2_SetTimerDelegate` (delegate `CustomEvent_0`))
  (`KismetSystemLibrary.Delay` 4.0)
  (`ActorComponent.Deactivate` (`self.NS_Fire`)))

(fn `UserConstructionScript`)