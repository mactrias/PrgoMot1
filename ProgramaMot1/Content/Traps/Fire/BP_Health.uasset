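; BP_Health is a healing zone actor with a fire effect that restores the third-person character's life while it stands inside.
; Entering the collider caches the character, activates NSFire1 and starts a looping timer that periodically calls HealFunc on the character's BPCLife component.
; Leaving stops the healing by re-setting the same timer event with zero time, then deactivates the effect after a short delay.
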(event `CustomEvent_0`
  (`/Game/ThirdPerson/Blueprints/BPC_life.HealFunc` (`/Game/ThirdPerson/Blueprints/BP_ThirdPersonCharacter.BPC_life` (stale `self.Collider.OnComponentBeginOverlap` _asbp_third_person_character)) 2.0))

(event `self.Collider.OnComponentBeginOverlap`
  (params (OverlappedComponent :type "PrimitiveComponent Object Reference") (OtherActor :type "Actor Object Reference") (OtherComp :type "PrimitiveComponent Object Reference") (OtherBodyIndex :type Integer) (bFromSweep :type Boolean) (SweepResult :type "HitResult Structure (by ref)"))
  (bind _asbp_third_person_character (cast `/Game/ThirdPerson/Blueprints/BP_ThirdPersonCharacter` OtherActor))
  (`ActorComponent.Activate` (`self.NS_Fire1`) false)
  (`KismetSystemLibrary.K2_SetTimerDelegate` (delegate `CustomEvent_0`) 0.5 true))

(event `self.Collider.OnComponentEndOverlap`
  (params (OverlappedComponent :type "PrimitiveComponent Object Reference") (OtherActor :type "Actor Object Reference") (OtherComp :type "PrimitiveComponent Object Reference") (OtherBodyIndex :type Integer))
  (cast `/Game/ThirdPerson/Blueprints/BP_ThirdPersonCharacter` OtherActor)
  (`KismetSystemLibrary.K2_SetTimerDelegate` (delegate `CustomEvent_0`))
  (`KismetSystemLibrary.Delay` 4.0)
  (`ActorComponent.Deactivate` (`self.NS_Fire1`)))

(fn `UserConstructionScript`)