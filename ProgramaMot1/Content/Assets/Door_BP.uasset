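; Interactive swinging door that the player opens and closes with the ActionBtn input.
; Overlapping the collision box with the third-person character enables input and shows two prompt components; leaving disables and hides them.
; A FlipFlop alternates playing and reversing a timeline that rotates the door mesh's yaw.
; Before opening, Doorpos uses a dot product of forward vector and direction to the player to pick the swing side, printing it.
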(event `InputAction|ActionBtn`
  (params (Key :type "Key Structure"))
  (:`Pressed`
    (`/Engine/EditorBlueprintResources/StandardMacros.FlipFlop`
      (:`A`
        (`self.doorpos`)
        (bind (_direction _newtrack_0) (`Timeline|Timeline_0` :`NewTime` 0.0 :!label _label)
          (:`Update`
            (`SceneComponent.K2_SetRelativeRotation` (`self.StaticMeshComponent1`) (`KismetMathLibrary.MakeRotator` 0.0 0.0 (* _newtrack_0 (`self.OpenAngle`))) false false))))
      (:`B`
        (goto _label :!via `Reverse`)))))

(event `self.colbox.OnComponentBeginOverlap`
  (params (OverlappedComponent :type "PrimitiveComponent Object Reference") (OtherActor :type "Actor Object Reference") (OtherComp :type "PrimitiveComponent Object Reference") (OtherBodyIndex :type Integer) (bFromSweep :type Boolean) (SweepResult :type "HitResult Structure (by ref)"))
  (cast `/Game/ThirdPerson/Blueprints/BP_ThirdPersonCharacter` OtherActor)
  (`self.EnableInput` (`GameplayStatics.GetPlayerController` 0))
  (`SceneComponent.SetHiddenInGame` (`self.opendoor`) false false)
  (`SceneComponent.SetHiddenInGame` (`self.opendoor1`) false false))

(event `self.colbox.OnComponentEndOverlap`
  (params (OverlappedComponent :type "PrimitiveComponent Object Reference") (OtherActor :type "Actor Object Reference") (OtherComp :type "PrimitiveComponent Object Reference") (OtherBodyIndex :type Integer))
  (cast `/Game/ThirdPerson/Blueprints/BP_ThirdPersonCharacter` OtherActor)
  (`self.DisableInput` (`GameplayStatics.GetPlayerController` 0))
  (`SceneComponent.SetHiddenInGame` (`self.opendoor`) true false)
  (`SceneComponent.SetHiddenInGame` (`self.opendoor1`) true false))

(fn `doorpos`
  (bind _returnvalue (`KismetMathLibrary.Dot_VectorVector` (`KismetMathLibrary.GetDirectionUnitVector` (`SceneComponent.GetSocketLocation` (`self.StaticMesh`) "None") (`self.K2_GetActorLocation` (`GameplayStatics.GetPlayerCharacter` 0))) (`self.GetActorForwardVector`)))
  (`KismetSystemLibrary.PrintString` (`KismetStringLibrary.Conv_DoubleToString` _returnvalue))
  (set `self.OpenAngle` (`KismetMathLibrary.SelectFloat` -80.0 80.0 (>= _returnvalue 0.0)))
  (return))

(fn `UserConstructionScript`)