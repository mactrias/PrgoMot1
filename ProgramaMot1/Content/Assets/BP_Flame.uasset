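; BP_Flame is a proximity-triggered flame effect that shows and hides a particle system for the player.
; BeginPlay caches the player as a BP_ThirdPersonCharacter, and the Box overlap events respond only to that reference.
; Entering the box shows the particles after a short delay, and leaving hides them after a longer one.
; It only toggles visibility and applies no damage.
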(event `self.ReceiveBeginPlay`
  (bind _asbp_third_person_character (cast `/Game/ThirdPerson/Blueprints/BP_ThirdPersonCharacter` (`GameplayStatics.GetPlayerCharacter` 0)))
  (set `self.Player_Ref` _asbp_third_person_character))

(event `self.Box.OnComponentBeginOverlap`
  (params (OverlappedComponent :type "PrimitiveComponent Object Reference") (OtherActor :type "Actor Object Reference") (OtherComp :type "PrimitiveComponent Object Reference") (OtherBodyIndex :type Integer) (bFromSweep :type Boolean) (SweepResult :type "HitResult Structure (by ref)"))
  (if (== OtherActor (`self.Player_Ref`))
    (`KismetSystemLibrary.Delay` 1.5)
    (`SceneComponent.SetVisibility` (`self.ParticleSystem`) true false)))

(event `self.Box.OnComponentEndOverlap`
  (params (OverlappedComponent :type "PrimitiveComponent Object Reference") (OtherActor :type "Actor Object Reference") (OtherComp :type "PrimitiveComponent Object Reference") (OtherBodyIndex :type Integer))
  (if (== OtherActor (`self.Player_Ref`))
    (`KismetSystemLibrary.Delay` 3.0)
    (`SceneComponent.SetVisibility` (`self.ParticleSystem`) false false)))

(fn `UserConstructionScript`)