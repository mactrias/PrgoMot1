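; Enemy character Blueprint that chases the player and plays an attack montage on arrival.
; Tick halts movement until PawnSensing sees a pawn and sets SeePlayer, which is never effectively cleared.
; Each sighting calls Follow, which re-arms CanAttack and uses AIMoveTo toward player 0, attempting the montage on success, though no montage asset is specified.
; Die is an empty stub.
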(event `self.ReceiveTick`
  (params (DeltaSeconds :type "Float (single-precision)"))
  (if (not (`self.seePlayer`))
    (`MovementComponent.StopMovementImmediately` (`self.CharacterMovement`))))

(event `self.PawnSensing.OnSeePawn`
  (params (Pawn :type "Pawn Object Reference"))
  (set `self.seePlayer` true)
  (`self.follow`))

(event `follow`
  (set `self.canAttack` true)
  (if (`self.seePlayer`)
    (`|AIMoveTo` self (0.0 0.0 0.0) (`GameplayStatics.GetPlayerCharacter` 0) 50.0
      (:`OnSuccess`
        (if (`self.canAttack`)
          (set `self.canAttack` false)
          (`self.PlayAnimMontage` null))))
    (else
      (set `self.seePlayer` false))))

(fn `Die`)

(fn `UserConstructionScript`)