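; BP_Ai is an AI enemy pawn that detects and attacks the third-person player character.
; When its PawnSensing component sees the player, it sets the hasSeenPlayer Blackboard flag on its AI controller.
; The AttackPlayer event sweeps a debug-drawn sphere trace forward for pawns and, on hitting the player, only prints "attacking", with no damage applied.
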(event `self.PawnSensing.OnSeePawn`
  (params (Pawn :type "Pawn Object Reference"))
  (cast `/Game/ThirdPerson/Blueprints/BP_ThirdPersonCharacter` Pawn)
  (`BlackboardComponent.SetValueAsBool` (`AIBlueprintHelperLibrary.GetBlackboard` (`AIBlueprintHelperLibrary.GetAIController` self)) "hasSeenPlayer" true))

(event `AttackPlayer`
  (bind _returnvalue (`self.K2_GetActorLocation`))
  (bind (_outhit _returnvalue_2) (`KismetSystemLibrary.SphereTraceSingleForObjects` :`Start` _returnvalue :`End` (+ _returnvalue (* (`KismetMathLibrary.GetForwardVector` (`self.K2_GetActorRotation`)) 300.0)) :`Radius` 120.0 :`ObjectTypes` (`|MakeArray` "ObjectTypeQuery3" :!type "EObjectTypeQuery Enum") :`DrawDebugType` "ForDuration"))
  (if _returnvalue_2
    (cast `/Game/ThirdPerson/Blueprints/BP_ThirdPersonCharacter` (`.HitActor` (`GameplayStatics.BreakHitResult` _outhit)))
    (`KismetSystemLibrary.PrintString` "attacking" true true (struct :`R` 1.0 :`B` 0.076939 :`A` 1.0))))

(fn `UserConstructionScript`)